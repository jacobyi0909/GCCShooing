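; BP_EnemyManager is a spawner actor that periodically creates BP_Enemy instances in the shooting game.
; On BeginPlay it picks a random interval between Min and Max, then Tick accumulates delta time until that interval is exceeded.
; It then spawns an enemy at its Arrow component's world transform, always spawning regardless of collision, rolls a new interval and resets the timer.
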(event `self.ReceiveBeginPlay`
  (`self.SetMakeTime`))

(event `self.ReceiveTick`
  (params (DeltaSeconds :type "Float (single-precision)"))
  (set `self.CurTime` (+ (`self.CurTime`) (`GameplayStatics.GetWorldDeltaSeconds`)))
  (if (> (`self.CurTime`) (`self.MakeTime`))
    (`self.MakeEnemy`)
    (`self.SetMakeTime`)
    (set `self.CurTime` 0.0)))

(fn `MakeEnemy`
  (`|SpawnActorFromClass` "/Game/Shooting/Blueprints/BP_Enemy.BP_Enemy_C" (`SceneComponent.K2_GetComponentToWorld` (`self.Arrow`)) "AlwaysSpawn" "MultiplyWithRoot" null null))

(fn `SetMakeTime`
  (set `self.MakeTime` (`KismetMathLibrary.RandomFloatInRange` (`self.Min`) (`self.Max`))))

(fn `UserConstructionScript`)