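; Player actor for a shooting game that moves in its right/up plane and fires bullets.
; Each Tick combines the Horizontal and Vertical values into a normalized direction, scaled by Speed and delta time, then applies a swept location change.
; Pressing the Fire input spawns a bullet at the FirePoint transform, regardless of collisions.
; A leftover rotation call is never executed.
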(event `self.ReceiveBeginPlay`)

(event `self.ReceiveTick`
  (params (DeltaSeconds :type "Float (single-precision)"))
  ; P
  (`self.K2_SetActorLocation` (+ (`self.K2_GetActorLocation`) (* (* (`KismetMathLibrary.Normal` (+ (* (`self.GetActorRightVector`) (`self.GetInputAxisValue`)) (* (`self.GetActorUpVector`) (`self.GetInputAxisValue`)))) (`self.Speed`)) (`GameplayStatics.GetWorldDeltaSeconds`))) true))

(event `InputAction|Fire`
  (params (Key :type "Key Structure"))
  ; 마우스 왼쪽 버튼을 누르면 총알을 생성해서 총구위치에 배치하고싶다.
  (:`Pressed`
    (`|SpawnActorFromClass` "/Game/Shooting/Blueprints/BP_Bullet.BP_Bullet_C" (`SceneComponent.K2_GetComponentToWorld` (`self.FirePoint`)) "AlwaysSpawn" "MultiplyWithRoot" null null)))

(fn `UserConstructionScript`)